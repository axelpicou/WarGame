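; Player-flown biplane pawn that drives a physics body (Driver) with Enhanced Input for throttle, roll, pitch and yaw.
; A looping timer steps AccelAmount while throttle input is held; Tick blends velocity toward forward times throttle and prints target speed.
; Axis inputs apply torque, with pitch scaled by throttle, while Tick adds counter-spin damping and constant downward force.
; A fast timer calls PropRudderElevator, currently an empty stub.
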(event `self.ReceiveBeginPlay`
  (cast `/Game/Blueprint/BP_biPlanePawn` self)
  (`EnhancedInputSubsystemInterface.AddMappingContext` (pcsubsystem `EnhancedInputLocalPlayerSubsystem` (`GameplayStatics.GetPlayerController` 0)) "/Game/Blueprint/INput/IMC_Plane.IMC_Plane" 0 (struct))
  (`KismetSystemLibrary.K2_SetTimerDelegate` (delegate `AccelChange`) 0.3 true)
  (`KismetSystemLibrary.K2_SetTimerDelegate` (delegate `Anim`) 0.01 true))

(event `EnhancedInput|/Game/Blueprint/INput/IA_accel`
  (params (ActionValue :type "Float (double-precision)") (ElapsedSeconds :type "Float (double-precision)") (TriggeredSeconds :type "Float (double-precision)") (InputAction :type "InputAction Object Reference" :default "/Game/Blueprint/INput/IA_accel.IA_accel"))
  (:`Triggered`
    (if (> ActionValue 0.0)
      (set `self.AccelUP` true)
      (else
        (set `self.AccelDown` true))))
  (:`Completed`
    (set `self.AccelUP` false)
    (set `self.AccelDown` false)))

(event `AccelChange`
  (`self.ThrottleInput`))

(event `Anim`
  (`self.PropRudderElevator`))

(event `EnhancedInput|/Game/Blueprint/INput/IA_Roll`
  (params (ActionValue :type "Float (double-precision)") (ElapsedSeconds :type "Float (double-precision)") (TriggeredSeconds :type "Float (double-precision)") (InputAction :type "InputAction Object Reference" :default "/Game/Blueprint/INput/IA_Roll.IA_Roll"))
  (:`Triggered`
    (`PrimitiveComponent.AddTorqueInDegrees` (`self.Driver`) (`KismetMathLibrary.VLerp` (0.0 0.0 0.0) (* (* ActionValue (`self.AirControl`)) (`SceneComponent.GetForwardVector` (`self.Driver`))) 0.1) "None" true)))

(event `EnhancedInput|/Game/Blueprint/INput/IA_MoveForward`
  (params (ActionValue :type "Float (double-precision)") (ElapsedSeconds :type "Float (double-precision)") (TriggeredSeconds :type "Float (double-precision)") (InputAction :type "InputAction Object Reference" :default "/Game/Blueprint/INput/IA_MoveForward.IA_MoveForward"))
  (:`Triggered`
    (`PrimitiveComponent.AddTorqueInDegrees` (`self.Driver`) (`KismetMathLibrary.VLerp` (0.0 0.0 0.0) (* (* ActionValue (* (`self.AirControlUpDown`) (/ (`self.AccelAmount`) 75))) (`SceneComponent.GetRightVector` (`self.Driver`))) 0.1) "None" true)))

(event `EnhancedInput|/Game/Blueprint/INput/IA_MoveRight`
  (params (ActionValue :type "Float (double-precision)") (ElapsedSeconds :type "Float (double-precision)") (TriggeredSeconds :type "Float (double-precision)") (InputAction :type "InputAction Object Reference" :default "/Game/Blueprint/INput/IA_MoveRight.IA_MoveRight"))
  (:`Triggered`
    (`PrimitiveComponent.AddTorqueInDegrees` (`self.Driver`) (`KismetMathLibrary.VLerp` (0.0 0.0 0.0) (* (* ActionValue (`self.AirControl`)) (`SceneComponent.GetUpVector` (`self.Driver`))) 0.1) "None" true)))

(event `self.ReceiveTick`
  (params (DeltaSeconds :type "Float (single-precision)"))
  (`PrimitiveComponent.AddTorqueInDegrees` (`self.Driver`) (/ (`KismetMathLibrary.NegateVector` (`PrimitiveComponent.GetPhysicsAngularVelocityInDegrees` (`self.Driver`) "None")) 0.5) "None" true)
  (`PrimitiveComponent.AddForce` (`self.Driver`) (0.0 0.0 -1500.0) "None" true)
  (`self.CalculateSpeed`)
  (`KismetSystemLibrary.PrintString` (`KismetStringLibrary.Conv_DoubleToString` (`self.ActualSpeed`))))

(fn `CalculateSpeed`
  (bind _driver (`self.Driver`))
  (bind _returnvalue (`KismetMathLibrary.Clamp` (* (`self.AccelAmount`) 250) 0 25000))
  (bind _returnvalue_2 (`PrimitiveComponent.GetPhysicsLinearVelocity` _driver "None"))
  (set `self.ActualSpeed` (`KismetMathLibrary.Conv_IntToDouble` _returnvalue))
  (`PrimitiveComponent.SetPhysicsLinearVelocity` (`self.Driver`) (`KismetMathLibrary.VLerp` _returnvalue_2 (* (`SceneComponent.GetForwardVector` _driver) _returnvalue) 0.01) false "None"))

(fn `PropRudderElevator`)

(fn `ThrottleInput`
  (bind _accelamount (`self.AccelAmount`))
  (if (`self.AccelUP`)
    (bind _result (`/Engine/EditorBlueprintResources/StandardMacros.IncrementInt` _accelamount)
      (:`  `
        (set `self.AccelAmount` (`KismetMathLibrary.Clamp` _result 0 100))))
    (elif (`self.AccelDown`)
      (bind _result_2 (`/Engine/EditorBlueprintResources/StandardMacros.DecrementInt` _accelamount)
        (:`  `
          (set `self.AccelAmount` (`KismetMathLibrary.Clamp` _result_2 0 100)))))))

(fn `UserConstructionScript`)