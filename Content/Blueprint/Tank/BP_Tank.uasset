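; Player-driven tank on Chaos wheeled vehicle movement, with Enhanced Input driving, speed/gear HUD and a menu key.
; Look input rotates the spring arm and updates turret yaw and clamped gun pitch; right-click toggles a gun-sight camera.
; Firing spawns a projectile, smoke and sound, then a recoil timeline torques the mesh.
; That timeline's update also decrements ammo and sets the reload timer each tick.
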(event `Key|P`
  (params (Key :type "Key Structure"))
  ;[1 1 1] Menu
  (:`Pressed`
    (bind _returnvalue (`|CreateWidget` "/Game/Menu/WB_Menu.WB_Menu_C"))
    (`UserWidget.AddToViewport` _returnvalue 0)))

(event `self.ReceiveBeginPlay`
  (bind _returnvalue (`GameplayStatics.GetPlayerController` 0))
  (`/Engine/EditorBlueprintResources/StandardMacros.IsValid` _returnvalue
    (:`Is Valid`
      (`EnhancedInputSubsystemInterface.AddMappingContext` (pcsubsystem `EnhancedInputLocalPlayerSubsystem` _returnvalue) "/Game/Blueprint/INput/Tank/IMC_Tank.IMC_Tank" 0 (struct))
      (bind _aschaos_wheeled_vehicle_movement_component (cast `ChaosWheeledVehicleMovementComponent` (`self.VehicleMovementComponent`)))
      (set `self.As Chaos Wheeled ` _aschaos_wheeled_vehicle_movement_component)
      (`self.Reload` (`self.ReloadMax`))
      (bind _returnvalue_2 (`|CreateWidget` "/Game/Blueprint/Tank/UI/VehicleUI.VehicleUI_C" _returnvalue))
      (bind _output_get (set `self.UI` _returnvalue_2))
      (`UserWidget.AddToViewport` _output_get 0))))

(event `self.ReceiveTick`
  (params (DeltaSeconds :type "Float (single-precision)"))
  ;[1 1 1] Ui
  (`/Game/Blueprint/Tank/UI/VehicleUI.UpdateSpeed` (`self.UI`) (`ChaosVehicleMovementComponent.GetForwardSpeed` (`self.VehicleMovementComponent`)))
  (`/Game/Blueprint/Tank/UI/VehicleUI.UpdateGear` (`self.UI`) (`ChaosVehicleMovementComponent.GetCurrentGear` (`self.VehicleMovementComponent`))))

(event `Set Turrent Yaw`
  (params (Yaw :type "Float (double-precision)"))
  ;[1 1 1] Turrent Anime
  (set `self.Turrent Yaw` (+ Yaw (`self.Turrent Yaw`))))

(event `Set Gun Pitch`
  (params (Pitch :type "Float (double-precision)"))
  ;[1 1 1] Gun Anime
  (set `self.Gun Pitch` (`KismetMathLibrary.FClamp` (+ (`self.Gun Pitch`) Pitch) (`self.Min GunPitch`) (`self.Max GunPitch`))))

(event `EnhancedInput|/Game/Blueprint/INput/Tank/Action/IA_Shoot`
  (params (ActionValue :type Boolean) (ElapsedSeconds :type "Float (double-precision)") (TriggeredSeconds :type "Float (double-precision)") (InputAction :type "InputAction Object Reference" :default "/Game/Blueprint/INput/Tank/Action/IA_Shoot.IA_Shoot"))
  (bind _spawnobu (`self.SpawnObu`))
  ;[1 1 1] Spanw projectile/reload
  (:`Triggered`
    (if ActionValue
      (if (> (`self.ReloadCurrent`) 0)
        (`self.Muzzle FX`)
        (`self.Shooting Sound`)
        (`|SpawnActorFromClass` "/Game/Blueprint/Projectile/BP_Projectile.BP_Projectile_C" (`KismetMathLibrary.MakeTransform` (`SceneComponent.K2_GetComponentLocation` _spawnobu) (`SceneComponent.K2_GetComponentRotation` _spawnobu)) "Undefined" "MultiplyWithRoot" self (`self.Instigator`))
        (bind (_direction _recoil) (`Timeline|Recoil` :!via `PlayFromStart`)
          (:`Update`
            (`self.Calculate Recoil` _recoil)
            (set `self.ReloadCurrent` (`KismetMathLibrary.Clamp` (- (`self.ReloadCurrent`) 1) 0 (`self.ReloadMax`)))
            (`KismetSystemLibrary.K2_SetTimerDelegate` (delegate `ReloadTime`) (`self.ReloadTimer`))))))))

(event `EnhancedInput|/Game/Blueprint/INput/Tank/Action/IA_LookAround`
  (params (ActionValue :type "Vector2D Structure") (ElapsedSeconds :type "Float (double-precision)") (TriggeredSeconds :type "Float (double-precision)") (InputAction :type "InputAction Object Reference" :default "/Game/Blueprint/INput/Tank/Action/IA_LookAround.IA_LookAround"))
  (bind _springarm (`self.SpringArm`))
  (bind (_relativerotation_roll _relativerotation_pitch _relativerotation_yaw) (`KismetMathLibrary.BreakRotator` (`SceneComponent.RelativeRotation` _springarm)))
  (bind _returnvalue (`KismetMathLibrary.FClamp` _relativerotation_pitch (`self.Min GunPitch`) (`self.Max GunPitch`)))
  ;[1 1 1] Vehicle Controlle
  (:`Triggered`
    (`SceneComponent.K2_AddRelativeRotation` (`self.SpringArm`) (`KismetMathLibrary.MakeRotator` 0.0 ActionValue_Y ActionValue_X) false false :!label _label)
    (`self.Set Turrent Yaw` ActionValue_X)
    (`SceneComponent.K2_SetRelativeRotation` _springarm (`KismetMathLibrary.MakeRotator` _relativerotation_roll _returnvalue _relativerotation_yaw) false false)
    (`self.Set Gun Pitch` _returnvalue))
  (:`Ongoing`
    (goto _label))
  (:`Canceled`
    (goto _label)))

(event `ReloadTime`
  ;[1 1 1] Spanw projectile/reload
  (`self.Reload` (`self.ReloadMax`)))

(event `Reload`
  (params (ReloadCurrent :type Integer))
  ;[1 1 1] Spanw projectile/reload
  (set `self.ReloadCurrent` ReloadCurrent))

(event `ReloadRack`
  (params (ReloadRackCurrent :type Integer))
  ;[1 1 1] Spanw projectile/reload
)

(event `EnhancedInput|/Game/Blueprint/INput/Tank/Action/IA_Throttle`
  (params (ActionValue :type "Float (double-precision)") (ElapsedSeconds :type "Float (double-precision)") (TriggeredSeconds :type "Float (double-precision)") (InputAction :type "InputAction Object Reference" :default "/Game/Blueprint/INput/Tank/Action/IA_Throttle.IA_Throttle"))
  (bind _as_chaos_wheeled_ (`self.As Chaos Wheeled `))
  ;[1 1 1] Vehicle Controlle
  (:`Triggered`
    (`ChaosVehicleMovementComponent.SetThrottleInput` _as_chaos_wheeled_ ActionValue :!label _label_2)
    (`ChaosVehicleMovementComponent.SetBrakeInput` _as_chaos_wheeled_ (* ActionValue -1.0)))
  (:`Ongoing`
    (goto _label_2))
  (:`Completed`
    (goto _label_2)))

(event `Calculate Recoil`
  (params (Recoil :type "Float (double-precision)"))
  ;[1 1 1] Recoil
  (bind _output_get (set `self.Recoil Alpha` Recoil))
  (`PrimitiveComponent.AddTorqueInRadians` (`self.Mesh`) (`KismetMathLibrary.TransformDirection` (`SceneComponent.GetSocketTransform` (`self.Mesh`) (`self.Socket Turret`) "RTS_World") (`KismetMathLibrary.MakeVector` 0.0 (* _output_get (`self.Recoil Value`)))) (`self.Socket root`) true))

(event `Muzzle FX`
  (bind _mesh (`self.Mesh`))
  ;[1 1 1] Muzzle
  (`NiagaraFunctionLibrary.SpawnSystemAttached` "/Game/Blueprint/Tank/Niagara/NS_SmokeShoot.NS_SmokeShoot" _mesh (`self.Socket gun`) (.location (`SceneComponent.GetSocketTransform` _mesh (`self.Socket gun`) "RTS_World")) (.rotation (`SceneComponent.GetSocketTransform` _mesh (`self.Socket gun`) "RTS_World")) "KeepWorldPosition"))

(event `EnhancedInput|/Game/Blueprint/INput/Tank/Action/IA_Turn`
  (params (ActionValue :type "Float (double-precision)") (ElapsedSeconds :type "Float (double-precision)") (TriggeredSeconds :type "Float (double-precision)") (InputAction :type "InputAction Object Reference" :default "/Game/Blueprint/INput/Tank/Action/IA_Turn.IA_Turn"))
  ;[1 1 1] Vehicle Controlle
  (:`Triggered`
    (`ChaosVehicleMovementComponent.SetYawInput` (`self.As Chaos Wheeled `) ActionValue :!label _label_3))
  (:`Ongoing`
    (goto _label_3))
  (:`Completed`
    (goto _label_3)))

(event `EnhancedInput|/Game/Blueprint/INput/Tank/Action/IA_Handbrake`
  (params (ActionValue :type Boolean) (ElapsedSeconds :type "Float (double-precision)") (TriggeredSeconds :type "Float (double-precision)") (InputAction :type "InputAction Object Reference" :default "/Game/Blueprint/INput/Tank/Action/IA_Handbrake.IA_Handbrake"))
  (bind _as_chaos_wheeled_ (`self.As Chaos Wheeled `))
  ;[1 1 1] Vehicle Controlle
  (:`Started`
    (`ChaosVehicleMovementComponent.SetHandbrakeInput` _as_chaos_wheeled_ true))
  (:`Completed`
    (`ChaosVehicleMovementComponent.SetHandbrakeInput` _as_chaos_wheeled_ false)))

(event `Key|RightMouseButton`
  (params (Key :type "Key Structure"))
  ;[1 1 1] Cam
  (:`Pressed`
    (if (`ActorComponent.IsActive` (`self.Camera`))
      (`ActorComponent.SetActive` (`self.Camera`) false false)
      (`ActorComponent.SetActive` (`self.CameraGun`) true false)
      (bind _returnvalue (`|CreateWidget` "/Game/Blueprint/Tank/Viser/WB_Viser.WB_Viser_C"))
      (`UserWidget.AddToViewport` _returnvalue 0)
      (elif (`ActorComponent.IsActive` (`self.CameraGun`))
        (`ActorComponent.SetActive` (`self.Camera`) true false)
        (`ActorComponent.SetActive` (`self.CameraGun`) false false)
        (`Widget.RemoveFromParent` _returnvalue)))))

(event `Shooting Sound`
  (bind _socket_gun (`self.Socket gun`))
  (bind _mesh (`self.Mesh`))
  ;[1 1 1] Sound Shooting
  (`GameplayStatics.SpawnSoundAtLocation` "/Game/Blueprint/Tank/SoundTank/GUNAuto_Coup_de_feu_de_beretta_m12_9_mm__ID_0437__LS.GUNAuto_Coup_de_feu_de_beretta_m12_9_mm__ID_0437__LS" (`SceneComponent.GetSocketLocation` _mesh _socket_gun) (`SceneComponent.GetSocketRotation` _mesh _socket_gun) 1.0 1.0 0.0 "/Game/Blueprint/Tank/SoundTank/ATT_explosion.ATT_explosion" null))

(fn `UserConstructionScript`)