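; Player plane with mouse-aim flight: mouse input rotates an aim rig, and the spring-arm camera damps toward it.
; Each tick an autopilot turns the aim point into yaw, pitch and roll, blending wing-leveling into banking by off-target angle.
; Roll input can override the autopilot, while pitch is currently always taken from MoveRight input.
; The results apply torque to the Driver body, with forward force from a timer-stepped throttle.
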(event `self.ReceiveTick`
  (params (DeltaSeconds :type "Float (single-precision)"))
  (set `self.DeltaSecond` DeltaSeconds)
  (`self.UpdatePhysics`))

(event `self.ReceiveBeginPlay`
  (cast `/Game/Blueprint/BP_PLayerPlane` self)
  (`EnhancedInputSubsystemInterface.AddMappingContext` (pcsubsystem `EnhancedInputLocalPlayerSubsystem` (`GameplayStatics.GetPlayerController` 0)) "/Game/Blueprint/INput/IMC_Plane.IMC_Plane" 0 (struct))
  (`KismetSystemLibrary.K2_SetTimerDelegate` (delegate `accel`) 0.5 true)
  (`SceneComponent.SetAbsolute` (`self.Controller_ROOT`) false true true))

(event `accel`
  (`self.Throttle`))

(event `EnhancedInput|/Game/Blueprint/INput/IA_accel`
  (params (ActionValue :type "Float (double-precision)") (ElapsedSeconds :type "Float (double-precision)") (TriggeredSeconds :type "Float (double-precision)") (InputAction :type "InputAction Object Reference" :default "/Game/Blueprint/INput/IA_accel.IA_accel"))
  (:`Triggered`
    (if (> ActionValue 0.0)
      (set `self.ThrottleUP` true)
      (else
        (set `self.ThrottleDown` true)))))

(event `EnhancedInput|/Game/Blueprint/INput/IA_MoveForward`
  (params (ActionValue :type "Float (double-precision)") (ElapsedSeconds :type "Float (double-precision)") (TriggeredSeconds :type "Float (double-precision)") (InputAction :type "InputAction Object Reference" :default "/Game/Blueprint/INput/IA_MoveForward.IA_MoveForward"))
  (:`Triggered`
    (`self.RotateRig` 0.0 (* ActionValue (`self.MouseSensitivity`)))))

(event `EnhancedInput|/Game/Blueprint/INput/IA_MoveRight`
  (params (ActionValue :type "Float (double-precision)") (ElapsedSeconds :type "Float (double-precision)") (TriggeredSeconds :type "Float (double-precision)") (InputAction :type "InputAction Object Reference" :default "/Game/Blueprint/INput/IA_MoveRight.IA_MoveRight"))
  (:`Triggered`
    (`self.RotateRig` (* ActionValue (`self.MouseSensitivity`)))))

(event `RotateRig`
  (params (InputX :type "Float (double-precision)") (InputY :type "Float (double-precision)"))
  (bind _springarm (`self.SpringArm`))
  (bind (_returnvalue_x _returnvalue_y _returnvalue_z) (`KismetMathLibrary.BreakVector` (`SceneComponent.GetForwardVector` (`self.ControllerAimScene`))))
  (`SceneComponent.K2_AddWorldRotation` (`self.ControllerAimScene`) (`KismetMathLibrary.RotatorFromAxisAndAngle` (`SceneComponent.GetUpVector` (`self.Camera`)) InputX) false false)
  (`SceneComponent.K2_AddWorldRotation` (`self.ControllerAimScene`) (`KismetMathLibrary.RotatorFromAxisAndAngle` (`SceneComponent.GetRightVector` (`self.Camera`)) InputY) false false)
  (bind _returnvalue (`self.GetControllerAimEndLocation`))
  (bind _returnvalue_2 (`self.Damp` (`SceneComponent.K2_GetComponentRotation` (`self.SpringArm`)) (`KismetMathLibrary.MakeRotFromXZ` (- _returnvalue (`SceneComponent.K2_GetComponentLocation` _springarm)) (select `bool` (> _returnvalue_z 0.9) :`false` (`KismetMathLibrary.MakeVector` 0.0 0.0 1.0) :`true` (`SceneComponent.GetUpVector` _springarm))) (`self.CameraSmooth`) (`self.DeltaSecond`) true))
  (`SceneComponent.K2_SetWorldRotation` (`self.SpringArm`) _returnvalue_2 false false))

(event `UpdatePhysics`
  (`self.UpdateAirCraftPhysic`))

(fn `CalculateSpeed`
  (bind _driver (`self.Driver`))
  (bind _returnvalue (`PrimitiveComponent.GetPhysicsLinearVelocity` _driver "None"))
  (`PrimitiveComponent.SetPhysicsLinearVelocity` (`self.Driver`) (`KismetMathLibrary.VLerp` _returnvalue (* (`SceneComponent.GetForwardVector` _driver) (`KismetMathLibrary.FClamp` (* (`self.ThrottleAmount`) 250) 0.0 25000.0)) 0.01) false "None"))

(fn `Damp`
  (params (A :type "Rotator Structure") (B :type "Rotator Structure") (Time :type "Float (double-precision)") (DeltaSeconds :type "Float (double-precision)") (ShortestPath :type Boolean))
  (returns (ReturnValue :type "Rotator Structure"))
  (return (`KismetMathLibrary.RLerp` A B (* (`KismetMathLibrary.Exp` (* Time DeltaSeconds -1.0)) 1.0) ShortestPath)))

(fn `GetBoresightEndLocation`
  (returns (ReturnValue :type "Vector Structure"))
  (return (+ (`self.K2_GetActorLocation`) (* (`self.GetActorForwardVector`) (`self.AimDistance`)))))

(fn `getBoresightStartLocation`
  (returns (ReturnValue :type "Vector Structure"))
  (return (`self.K2_GetActorLocation`)))

(fn `GetControllerAimEndLocation`
  (returns (ReturnValue :type "Vector Structure"))
  (bind _controlleraimscene (`self.ControllerAimScene`))
  (return (+ (`SceneComponent.K2_GetComponentLocation` _controlleraimscene) (* (`SceneComponent.GetForwardVector` _controlleraimscene) (`self.AimDistance`)))))

(fn `GetControllerAimStartLocation`
  (returns (ReturnValue :type "Vector Structure"))
  (return (`SceneComponent.K2_GetComponentLocation` (`self.ControllerAimScene`))))

(fn `RunAutopilot`
  (params (FlyTarget :type "Vector Structure") (OutYaw :type "Float (double-precision)") (OutPitch :type "Float (double-precision)") (OutRoll :type "Float (double-precision)"))
  (locals (LocalFlyTarget :type "Vector Structure") (AngleOfTarget :type "Float (double-precision)") (AggressiveRoll :type "Float (double-precision)") (WingLevelRoll :type "Float (double-precision)") (WingLevelInfluence :type "Float (double-precision)"))
  (bind (_returnvalue_x _returnvalue_y _returnvalue_z) (`KismetMathLibrary.BreakVector` (`self.GetActorRightVector`)))
  (bind (_localflytarget_x _localflytarget_y _localflytarget_z) (`KismetMathLibrary.BreakVector` (`local.LocalFlyTarget`)))
  (bind (_localflytarget_x_2 _localflytarget_y_2) (`KismetMathLibrary.BreakVector` (`local.LocalFlyTarget`)))
  (`|ExecutionSequence`
    (:`then_0`
      (set `local.LocalFlyTarget` (* (`KismetMathLibrary.Normal` (`KismetMathLibrary.InverseTransformLocation` (`self.GetTransform`) (`local.FlyTarget`))) (`self.Sensivity`)))
      (set `local.AngleOfTarget` (`KismetMathLibrary.DegAcos` (`KismetMathLibrary.Dot_VectorVector` (`self.GetActorForwardVector`) (`KismetMathLibrary.Normal` (- (`local.FlyTarget`) (`self.K2_GetActorLocation`)))))))
    (:`then_1`
      (`|VariableSetRef` OutYaw (`KismetMathLibrary.FClamp` _localflytarget_y -1.0))
      (`|VariableSetRef` OutPitch (`KismetMathLibrary.FClamp` _localflytarget_z -1.0)))
    (:`then_2`
      (set `local.AggressiveRoll` (`KismetMathLibrary.FClamp` _localflytarget_y_2 -1.0))
      (set `local.WingLevelRoll` _returnvalue_z)
      (set `local.WingLevelInfluence` (`KismetMathLibrary.FClamp` (`KismetMathLibrary.NormalizeToRange` (`local.AngleOfTarget`) 0.0 (`self.AggressiveTurnAngle`))))
      (`|VariableSetRef` OutRoll (`KismetMathLibrary.Lerp` (`local.WingLevelRoll`) (`local.AggressiveRoll`) (`local.WingLevelInfluence`))))))

(fn `Throttle`
  (bind _throttleamount (`self.ThrottleAmount`))
  (if (`self.ThrottleUP`)
    (bind _result (`/Engine/EditorBlueprintResources/StandardMacros.IncrementInt` _throttleamount)
      (:`  `
        (bind _output_get (set `self.ThrottleAmount` (`KismetMathLibrary.Clamp` _result 0 100)))
        (`KismetSystemLibrary.PrintString` (`KismetStringLibrary.Conv_IntToString` _output_get))))
    (elif (`self.ThrottleDown`)
      (bind _result_2 (`/Engine/EditorBlueprintResources/StandardMacros.DecrementInt` _throttleamount)
        (:`  `
          (bind _output_get_2 (set `self.ThrottleAmount` (`KismetMathLibrary.Clamp` _result_2 0 100)))
          (`KismetSystemLibrary.PrintString` (`KismetStringLibrary.Conv_IntToString` _output_get_2)))))))

(fn `UpdateAirCraftPhysic`
  (locals (RollOverride :type Boolean) (PitchOverride :type Boolean) (AutoYaw :type "Float (double-precision)") (AutoPitch :type "Float (double-precision)") (AutoRoll :type "Float (double-precision)") (CurrentYaw :type "Float (double-precision)") (CurrentPitch :type "Float (double-precision)") (CurrentRoll :type "Float (double-precision)"))
  (`|ExecutionSequence`
    (:`then_0`
      (set `local.RollOverride` false)
      (set `local.PitchOverride` false)
      (set `local.AutoPitch` 0.0)
      (set `local.AutoYaw` 0.0)
      (set `local.AutoRoll` 0.0))
    (:`then_1`
      (`|ExecutionSequence`
        (:`then_0`
          (if (> (`KismetMathLibrary.Abs` (`|GetInputActionValue`)) 0.25)
            (set `local.RollOverride` true)))
        (:`then_1`
          (if true
            (set `local.RollOverride` (> (`KismetMathLibrary.Abs` (`|GetInputActionValue`)) 0.25))
            (set `local.PitchOverride` true)))))
    (:`then_2`
      (bind _returnvalue (`self.GetControllerAimEndLocation`))
      (`self.RunAutopilot` _returnvalue (`local.AutoYaw`) (`local.AutoPitch`) (`local.AutoRoll`)))
    (:`then_3`
      (set `local.CurrentYaw` (`local.AutoYaw`))
      (set `local.CurrentPitch` (select `bool` (`local.PitchOverride`) :`false` (`local.AutoPitch`) :`true` (`|GetInputActionValue`)))
      (set `local.CurrentRoll` (`KismetMathLibrary.SelectFloat` (`local.AutoRoll`) (`|GetInputActionValue`) (`local.RollOverride`))))
    (:`then_4`
      (`|ExecutionSequence`
        (:`then_0`
          (`PrimitiveComponent.AddForce` (`self.Driver`) (* (`self.GetActorForwardVector`) (* (`self.ThrottleAmount`) (`self.ForceMultiplier`))) "None" false))
        (:`then_1`
          (`PrimitiveComponent.AddTorqueInRadians` (`self.Driver`) (* (`KismetMathLibrary.TransformDirection` (`self.GetTransform`) (* (`self.Turntorque`) (`KismetMathLibrary.MakeVector` (`local.CurrentRoll`) (`local.CurrentPitch`) (`local.CurrentYaw`)))) (`self.ForceMultiplier`)) "None" false))))))

(fn `UserConstructionScript`)