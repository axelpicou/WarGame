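; BP_MainMenuPlane is a jet for the main menu, built as a set of flight and animation functions with no event graph calling them.
; Throttle flags step AccelAmount, which drives the thruster effects and blends the Driver's physics velocity toward its forward vector.
; Yaw, pitch and roll functions ease rudders, flaps, elevators and ailerons toward input, with Reset variants easing to neutral.
; Their deflection fractions scale AirControl into per-axis control values.
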(fn `CalculateAirControl`
  (returns (Yawcontrol :type "Float (double-precision)") (RollControll :type "Float (double-precision)") (PitchControl :type "Float (double-precision)"))
  (return (* (`self.AirControl`) (`self.percentageYaw`)) (* (`self.PercentageRoll`) (`self.AirControl`)) (* (`self.PercentagePitch`) (`self.AirControl`))))

(fn `CalculateSpeed`
  (bind _driver (`self.Driver`))
  (bind _returnvalue (`PrimitiveComponent.GetPhysicsLinearVelocity` _driver "None"))
  (`PrimitiveComponent.SetPhysicsLinearVelocity` (`self.Driver`) (`KismetMathLibrary.VLerp` _returnvalue (* (`SceneComponent.GetForwardVector` _driver) (`KismetMathLibrary.Clamp` (* (`self.AccelAmount`) 250) 0 25000)) 0.01) false "None"))

(fn `PItchAnimation`
  (params (DeltaSecond :type "Float (double-precision)") (Pitch :type "Float (double-precision)"))
  (bind _maxelevatorpitch (`self.MaxElevatorPitch`))
  (bind _maxflapptich (`self.MaxFlapPtich`))
  (bind _returnvalue (`KismetMathLibrary.MapRangeClamped` (`self.CurrentPitch`) -1.0 1.0 _maxelevatorpitch (`self.Negate` _maxelevatorpitch)))
  (bind _returnvalue_2 (`KismetMathLibrary.MapRangeClamped` (`self.CurrentPitch`) -1.0 1.0 _maxflapptich (`self.Negate` _maxflapptich)))
  (bind _out (`self.Negate` _returnvalue))
  (set `self.TargetPitch` Pitch)
  (set `self.CurrentPitch` (`KismetMathLibrary.FInterpTo` (`self.CurrentPitch`) (`self.TargetPitch`) (`GameplayStatics.GetWorldDeltaSeconds`) 10.0))
  (`SceneComponent.K2_SetRelativeRotation` (`self.FlapL`) (`KismetMathLibrary.MakeRotator` 0.0 _returnvalue_2) false false)
  (`SceneComponent.K2_SetRelativeRotation` (`self.FlapR`) (`KismetMathLibrary.MakeRotator` 0.0 _returnvalue_2) false false)
  (`SceneComponent.K2_SetRelativeRotation` (`self.ElevatorL`) (`KismetMathLibrary.MakeRotator` 0.0 _out) false false)
  (`SceneComponent.K2_SetRelativeRotation` (`self.ElevatorR`) (`KismetMathLibrary.MakeRotator` 0.0 _out) false false)
  (set `self.PercentagePitch` (`KismetMathLibrary.Abs` (/ (/ (* _returnvalue 100.0) (`self.MaxElevatorPitch`)) 100.0))))

(fn `Reset Aileron`
  (bind _maxaileronptich (`self.MaxAileronPtich`))
  (bind _maxaileronptich_2 (`self.MaxAileronPtich`))
  (bind _returnvalue (`KismetMathLibrary.MapRangeClamped` (`self.CurrentRoll`) -1.0 1.0 _maxaileronptich_2 (`self.Negate` _maxaileronptich_2)))
  (set `self.TargetRoll` 0.0)
  (set `self.CurrentRoll` (`KismetMathLibrary.FInterpTo` (`self.CurrentRoll`) (`self.TargetRoll`) (`GameplayStatics.GetWorldDeltaSeconds`) 10.0))
  (`SceneComponent.K2_SetRelativeRotation` (`self.aileronL`) (`KismetMathLibrary.MakeRotator` 0.0 (`KismetMathLibrary.MapRangeClamped` (`self.CurrentRoll`) -1.0 1.0 _maxaileronptich (`self.Negate` _maxaileronptich))) false false)
  (`SceneComponent.K2_SetRelativeRotation` (`self.AileronR`) (`KismetMathLibrary.MakeRotator` 0.0 (`self.Negate` _returnvalue)) false false)
  (set `self.PercentageRoll` (`KismetMathLibrary.Abs` (/ (/ (* _returnvalue 100.0) (`self.MaxAileronPtich`)) 100.0))))

(fn `ResetElevator`
  (bind _maxelevatorpitch (`self.MaxElevatorPitch`))
  (bind _maxflapptich (`self.MaxFlapPtich`))
  (bind _returnvalue (`KismetMathLibrary.MapRangeClamped` (`self.CurrentPitch`) -1.0 1.0 _maxelevatorpitch (`self.Negate` _maxelevatorpitch)))
  (bind _returnvalue_2 (`KismetMathLibrary.MapRangeClamped` (`self.CurrentPitch`) -1.0 1.0 _maxflapptich (`self.Negate` _maxflapptich)))
  (bind _out (`self.Negate` _returnvalue))
  (set `self.TargetPitch` 0.0)
  (set `self.CurrentPitch` (`KismetMathLibrary.FInterpTo` (`self.CurrentPitch`) (`self.TargetPitch`) (`GameplayStatics.GetWorldDeltaSeconds`) 10.0))
  (`SceneComponent.K2_SetRelativeRotation` (`self.FlapL`) (`KismetMathLibrary.MakeRotator` 0.0 _returnvalue_2) false false)
  (`SceneComponent.K2_SetRelativeRotation` (`self.FlapR`) (`KismetMathLibrary.MakeRotator` 0.0 _returnvalue_2) false false)
  (`SceneComponent.K2_SetRelativeRotation` (`self.ElevatorL`) (`KismetMathLibrary.MakeRotator` 0.0 _out) false false)
  (`SceneComponent.K2_SetRelativeRotation` (`self.ElevatorR`) (`KismetMathLibrary.MakeRotator` 0.0 _out) false false)
  (set `self.PercentagePitch` (`KismetMathLibrary.Abs` (/ (/ (* _returnvalue 100.0) (`self.MaxElevatorPitch`)) 100.0))))

(fn `ResetRudder`
  (bind _returnvalue (`KismetMathLibrary.MapRangeClamped` (`self.CurrentYaw`) -1.0 1.0 (`self.maxRudderYaw`) (`self.Negate` (`self.maxRudderYaw`))))
  (set `self.TargetYaw` 0.0)
  (set `self.CurrentYaw` (`KismetMathLibrary.FInterpTo` (`self.CurrentYaw`) (`self.TargetYaw`) (`GameplayStatics.GetWorldDeltaSeconds`) 10.0))
  (`SceneComponent.K2_SetRelativeRotation` (`self.RudderL`) (`KismetMathLibrary.MakeRotator` 0.0 0.0 _returnvalue) false false)
  (`SceneComponent.K2_SetRelativeRotation` (`self.RudderR`) (`KismetMathLibrary.MakeRotator` 0.0 0.0 _returnvalue) false false)
  (set `self.percentageYaw` (`KismetMathLibrary.Abs` (/ (/ (* _returnvalue 100.0) (`self.maxRudderYaw`)) 100.0))))

(fn `RollAnimation`
  (params (DeltaSecond :type "Float (double-precision)") (Roll :type "Float (double-precision)"))
  (bind _maxaileronptich (`self.MaxAileronPtich`))
  (bind _maxaileronptich_2 (`self.MaxAileronPtich`))
  (bind _returnvalue (`KismetMathLibrary.MapRangeClamped` (`self.CurrentRoll`) -1.0 1.0 _maxaileronptich_2 (`self.Negate` _maxaileronptich_2)))
  (set `self.TargetRoll` Roll)
  (set `self.CurrentRoll` (`KismetMathLibrary.FInterpTo` (`self.CurrentRoll`) (`self.TargetRoll`) (`GameplayStatics.GetWorldDeltaSeconds`) 10.0))
  (`SceneComponent.K2_SetRelativeRotation` (`self.aileronL`) (`KismetMathLibrary.MakeRotator` 0.0 (`KismetMathLibrary.MapRangeClamped` (`self.CurrentRoll`) -1.0 1.0 _maxaileronptich (`self.Negate` _maxaileronptich))) false false)
  (`SceneComponent.K2_SetRelativeRotation` (`self.AileronR`) (`KismetMathLibrary.MakeRotator` 0.0 (`self.Negate` _returnvalue)) false false)
  (set `self.PercentageRoll` (`KismetMathLibrary.Abs` (/ (/ (* _returnvalue 100.0) (`self.MaxAileronPtich`)) 100.0))))

(fn `ThrottleInput`
  (bind _accelamount (`self.AccelAmount`))
  (if (`self.AccelUP`)
    (bind _result (`/Engine/EditorBlueprintResources/StandardMacros.IncrementInt` _accelamount)
      (:`  `
        (set `self.AccelAmount` (`KismetMathLibrary.Clamp` _result 0 100))))
    (elif (`self.AccelDown`)
      (bind _result_2 (`/Engine/EditorBlueprintResources/StandardMacros.DecrementInt` _accelamount)
        (:`  `
          (set `self.AccelAmount` (`KismetMathLibrary.Clamp` _result_2 0 100)))))))

(fn `UpdateThruster`
  (`NiagaraComponent.SetVariableVec3` (`self.LeftThrusterEffect`) "Attractor Position Offset" (`KismetMathLibrary.MakeVector` (`KismetMathLibrary.MapRangeClamped` (`KismetMathLibrary.Conv_IntToDouble` (`self.AccelAmount`)) 0.0 100.0 0.0 -500.0)))
  (`NiagaraComponent.SetVariableVec3` (`self.RightThrusterEffect`) "Attractor Position Offset" (`KismetMathLibrary.MakeVector` (`KismetMathLibrary.MapRangeClamped` (`KismetMathLibrary.Conv_IntToDouble` (`self.AccelAmount`)) 0.0 100.0 0.0 -500.0))))

(fn `UserConstructionScript`)

(fn `YawAnimation`
  (params (DeltaSecond :type "Float (double-precision)") (Yaw :type "Float (double-precision)"))
  (bind _returnvalue (`KismetMathLibrary.MapRangeClamped` (`self.CurrentYaw`) -1.0 1.0 (`self.maxRudderYaw`) (`self.Negate` (`self.maxRudderYaw`))))
  (set `self.TargetYaw` Yaw)
  (set `self.CurrentYaw` (`KismetMathLibrary.FInterpTo` (`self.CurrentYaw`) (`self.TargetYaw`) (`GameplayStatics.GetWorldDeltaSeconds`) 10.0))
  (`SceneComponent.K2_SetRelativeRotation` (`self.RudderL`) (`KismetMathLibrary.MakeRotator` 0.0 0.0 _returnvalue) false false)
  (`SceneComponent.K2_SetRelativeRotation` (`self.RudderR`) (`KismetMathLibrary.MakeRotator` 0.0 0.0 _returnvalue) false false)
  (set `self.percentageYaw` (`KismetMathLibrary.Abs` (/ (/ (* _returnvalue 100.0) (`self.maxRudderYaw`)) 100.0))))