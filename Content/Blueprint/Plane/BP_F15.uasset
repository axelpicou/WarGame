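; Player-flyable F-15 with Enhanced Input flight controls, a stat HUD and a pause menu.
; A timer steps throttle, while Tick blends physics velocity toward forward thrust and applies gravity and angular damping.
; Inputs animate control surfaces and apply torque, scaled by deflection for roll and yaw and by throttle for pitch.
; Tick also recenters surfaces, drives engine audio from throttle and speed, and updates Niagara thruster effects.
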(event `UIManager`
  (bind _returnvalue (`|CreateWidget` "/Game/Widget/Bp_Stat.Bp_Stat_C"))
  (`UserWidget.AddToViewport` _returnvalue 0))

(event `EnhancedInput|/Game/Blueprint/Plane/INput/Plane/IA_accel`
  (params (ActionValue :type "Float (double-precision)") (ElapsedSeconds :type "Float (double-precision)") (TriggeredSeconds :type "Float (double-precision)") (InputAction :type "InputAction Object Reference" :default "/Game/Blueprint/Plane/INput/Plane/IA_accel.IA_accel"))
  ;[1 0 0] input
  ;;[1 1 1] Acceleration up/down
  (:`Triggered`
    (if (> ActionValue 0.0)
      (set `self.AccelUP` true)
      (else
        (set `self.AccelDown` true))))
  (:`Completed`
    (set `self.AccelUP` false)
    (set `self.AccelDown` false)))

(event `self.ReceiveBeginPlay`
  ;[1 1 1] get IMC
  (`self.UIManager`)
  (cast `/Game/Blueprint/Plane/BP_F15` self)
  (`EnhancedInputSubsystemInterface.AddMappingContext` (pcsubsystem `EnhancedInputLocalPlayerSubsystem` (`GameplayStatics.GetPlayerController` 0)) "/Game/Blueprint/Plane/INput/Plane/IMC_Plane.IMC_Plane" 0 (struct))
  ;[1 1 1] Particle
  (bind _returnvalue (`NiagaraFunctionLibrary.SpawnSystemAttached` "/Game/Blueprint/Plane/Particle/NE_trusterEmiter_System.NE_trusterEmiter_System" (`self.Fuselage`) "ThrusterL" (0.0 0.0 0.0) (struct) "SnapToTargetIncludingScale"))
  (set `self.LeftThrusterEffect` _returnvalue)
  (bind _returnvalue_2 (`NiagaraFunctionLibrary.SpawnSystemAttached` "/Game/Blueprint/Plane/Particle/NE_trusterEmiter_System.NE_trusterEmiter_System" (`self.Fuselage`) "ThrusterR" (0.0 0.0 0.0) (struct) "SnapToTargetIncludingScale"))
  (set `self.RightThrusterEffect` _returnvalue_2)
  ;[1 0 0] input
  ;;[1 1 1] Acceleration up/down
  (`KismetSystemLibrary.K2_SetTimerDelegate` (delegate `AccelChange`) 0.3 true))

(event `AccelChange`
  ;[1 0 0] input
  ;;[1 1 1] Acceleration up/down
  (`self.ThrottleInput`))

(event `self.ReceiveTick`
  (params (DeltaSeconds :type "Float (single-precision)"))
  ;[1 1 1] Drag and gravity
  (`PrimitiveComponent.AddTorqueInDegrees` (`self.Driver`) (/ (`KismetMathLibrary.NegateVector` (`PrimitiveComponent.GetPhysicsAngularVelocityInDegrees` (`self.Driver`) "None")) 0.5) "None" true)
  (`PrimitiveComponent.AddForce` (`self.Driver`) (0.0 0.0 -1500.0) "None" true)
  ;[1 0 0] Physic
  (`self.CalculateSpeed`)
  ;;[1 1 1] Angular Drag
  (set `self.ActualSpeed` (`KismetMathLibrary.VSize` (`self.GetVelocity`)))
  (`PrimitiveComponent.SetAngularDamping` (`self.Fuselage`) (`KismetMathLibrary.FClamp` (/ (`self.ActualSpeed`) 4000.0) 0.01 15.0))
  (`self.Sound Management`)
  ;[1 1 1] Particle
  (`self.UpdateThruster`)
  ;[1 1 1] Reset Flap
  (`|ExecutionSequence`
    (:`then_0`
      (if (not (`self.Rolling`))
        (`self.Reset Aileron`)))
    (:`then_1`
      (if (not (`self.MoveRight`))
        (`self.ResetRudder`)))
    (:`then_2`
      (if (not (`self.MoveRight`))
        (`self.ResetElevator`)))))

(event `EnhancedInput|/Game/Blueprint/Plane/INput/Plane/IA_Roll`
  (params (ActionValue :type "Float (double-precision)") (ElapsedSeconds :type "Float (double-precision)") (TriggeredSeconds :type "Float (double-precision)") (InputAction :type "InputAction Object Reference" :default "/Game/Blueprint/Plane/INput/Plane/IA_Roll.IA_Roll"))
  ;[1 0 0] input
  ;;[1 1 1] roulie gauche/droit
  (:`Triggered`
    (`self.RollAnimation` (`GameplayStatics.GetWorldDeltaSeconds`) ActionValue)
    (bind (_yawcontrol _rollcontroll) (`self.CalculateAirControl`))
    (`PrimitiveComponent.AddTorqueInDegrees` (`self.Driver`) (`KismetMathLibrary.VLerp` (0.0 0.0 0.0) (* (* ActionValue _rollcontroll) (`SceneComponent.GetForwardVector` (`self.Driver`))) (`self.Alpha`)) "None" true)
    (set `self.Rolling` true))
  (:`Completed`
    (set `self.Rolling` false)))

(event `Sound Management`
  (bind _jetengineaudio (`self.jetEngineAudio`))
  (bind _actualspeed (`self.ActualSpeed`))
  (bind _jetengineaudio_2 (`self.jetEngineAudio`))
  ;[1 0 0] Volume Manager
  ;;[1 1 1] engine pitch
  (`AudioComponent.SetPitchMultiplier` _jetengineaudio_2 (`KismetMathLibrary.FInterpTo` (`AudioComponent.PitchMultiplier` _jetengineaudio_2) (`KismetMathLibrary.Conv_IntToDouble` (`self.AccelAmount`)) (`GameplayStatics.GetWorldDeltaSeconds`) 3.0))
  ;;[1 1 1] engineVolume
  (`AudioComponent.SetVolumeMultiplier` _jetengineaudio (`KismetMathLibrary.FClamp` (`KismetMathLibrary.FInterpTo` (`AudioComponent.VolumeMultiplier` _jetengineaudio) (`KismetMathLibrary.SelectFloat` 1.0 (/ _actualspeed 1000.0) (<= _actualspeed 9000.0)) (`GameplayStatics.GetWorldDeltaSeconds`) 3.0) 0.0 0.05))
  ;[1 0 0] Physic
  ;;[1 1 1] Movement Limiter
  (if (<= (`self.ActualSpeed`) 400.0)
    (set `self.Alpha` 0.01)
    (else
      (set `self.Alpha` 0.1))))

(event `EnhancedInput|/Game/Blueprint/Plane/INput/Plane/IA_MoveRight`
  (params (ActionValue :type "Float (double-precision)") (ElapsedSeconds :type "Float (double-precision)") (TriggeredSeconds :type "Float (double-precision)") (InputAction :type "InputAction Object Reference" :default "/Game/Blueprint/Plane/INput/Plane/IA_MoveRight.IA_MoveRight"))
  ;[1 0 0] input
  ;;[1 1 1] tourné gauche droite
  (:`Triggered`
    (`self.YawAnimation` (`GameplayStatics.GetWorldDeltaSeconds`) ActionValue)
    (bind _yawcontrol (`self.CalculateAirControl`))
    (`PrimitiveComponent.AddTorqueInDegrees` (`self.Driver`) (`KismetMathLibrary.VLerp` (0.0 0.0 0.0) (* (* ActionValue _yawcontrol) (`SceneComponent.GetUpVector` (`self.Driver`))) (`self.Alpha`)) "None" true)
    (set `self.MoveRight` true))
  (:`Completed`
    (set `self.MoveRight` false)))

(event `Key|P`
  (params (Key :type "Key Structure"))
  ;[1 1 1] Menu
  (:`Pressed`
    (bind _returnvalue (`|CreateWidget` "/Game/Menu/WB_Menu.WB_Menu_C"))
    (`UserWidget.AddToViewport` _returnvalue 0)
    (`GameplayStatics.SetGamePaused` true)))

(event `EnhancedInput|/Game/Blueprint/Plane/INput/Plane/IA_MoveForward`
  (params (ActionValue :type "Float (double-precision)") (ElapsedSeconds :type "Float (double-precision)") (TriggeredSeconds :type "Float (double-precision)") (InputAction :type "InputAction Object Reference" :default "/Game/Blueprint/Plane/INput/Plane/IA_MoveForward.IA_MoveForward"))
  ;[1 0 0] input
  ;;[1 1 1] monté baissé le nez
  (:`Triggered`
    (`self.PItchAnimation` (`GameplayStatics.GetWorldDeltaSeconds`) ActionValue)
    (`PrimitiveComponent.AddTorqueInDegrees` (`self.Driver`) (`KismetMathLibrary.VLerp` (0.0 0.0 0.0) (* (* ActionValue (* (`self.AirControl`) (/ (`self.AccelAmount`) 75))) (`SceneComponent.GetRightVector` (`self.Driver`))) 0.1) "None" true)
    (set `self.MoveForward` true))
  (:`Completed`
    (set `self.MoveForward` false)))

(fn `CalculateAirControl`
  (returns (Yawcontrol :type "Float (double-precision)") (RollControll :type "Float (double-precision)") (PitchControl :type "Float (double-precision)"))
  (return (* (`self.AirControl`) (`self.percentageYaw`)) (* (`self.PercentageRoll`) (`self.AirControl`)) (* (`self.PercentagePitch`) (`self.AirControl`))))

(fn `CalculateSpeed`
  (bind _driver (`self.Driver`))
  (bind _returnvalue (`PrimitiveComponent.GetPhysicsLinearVelocity` _driver "None"))
  (`PrimitiveComponent.SetPhysicsLinearVelocity` (`self.Driver`) (`KismetMathLibrary.VLerp` _returnvalue (* (`SceneComponent.GetForwardVector` _driver) (`KismetMathLibrary.Clamp` (* (`self.AccelAmount`) 250) 0 25000)) 0.01) false "None"))

(fn `PItchAnimation`
  (params (DeltaSecond :type "Float (double-precision)") (Pitch :type "Float (double-precision)"))
  (bind _maxelevatorpitch (`self.MaxElevatorPitch`))
  (bind _maxflapptich (`self.MaxFlapPtich`))
  (bind _returnvalue (`KismetMathLibrary.MapRangeClamped` (`self.CurrentPitch`) -1.0 1.0 _maxelevatorpitch (`self.Negate` _maxelevatorpitch)))
  (bind _returnvalue_2 (`KismetMathLibrary.MapRangeClamped` (`self.CurrentPitch`) -1.0 1.0 _maxflapptich (`self.Negate` _maxflapptich)))
  (bind _out (`self.Negate` _returnvalue))
  (set `self.TargetPitch` Pitch)
  (set `self.CurrentPitch` (`KismetMathLibrary.FInterpTo` (`self.CurrentPitch`) (`self.TargetPitch`) (`GameplayStatics.GetWorldDeltaSeconds`) 10.0))
  (`SceneComponent.K2_SetRelativeRotation` (`self.FlapL`) (`KismetMathLibrary.MakeRotator` 0.0 _returnvalue_2) false false)
  (`SceneComponent.K2_SetRelativeRotation` (`self.FlapR`) (`KismetMathLibrary.MakeRotator` 0.0 _returnvalue_2) false false)
  (`SceneComponent.K2_SetRelativeRotation` (`self.ElevatorL`) (`KismetMathLibrary.MakeRotator` 0.0 _out) false false)
  (`SceneComponent.K2_SetRelativeRotation` (`self.ElevatorR`) (`KismetMathLibrary.MakeRotator` 0.0 _out) false false)
  (set `self.PercentagePitch` (`KismetMathLibrary.Abs` (/ (/ (* _returnvalue 100.0) (`self.MaxElevatorPitch`)) 100.0))))

(fn `Reset Aileron`
  (bind _maxaileronptich (`self.MaxAileronPtich`))
  (bind _maxaileronptich_2 (`self.MaxAileronPtich`))
  (bind _returnvalue (`KismetMathLibrary.MapRangeClamped` (`self.CurrentRoll`) -1.0 1.0 _maxaileronptich_2 (`self.Negate` _maxaileronptich_2)))
  (set `self.TargetRoll` 0.0)
  (set `self.CurrentRoll` (`KismetMathLibrary.FInterpTo` (`self.CurrentRoll`) (`self.TargetRoll`) (`GameplayStatics.GetWorldDeltaSeconds`) 10.0))
  (`SceneComponent.K2_SetRelativeRotation` (`self.aileronL`) (`KismetMathLibrary.MakeRotator` 0.0 (`KismetMathLibrary.MapRangeClamped` (`self.CurrentRoll`) -1.0 1.0 _maxaileronptich (`self.Negate` _maxaileronptich))) false false)
  (`SceneComponent.K2_SetRelativeRotation` (`self.AileronR`) (`KismetMathLibrary.MakeRotator` 0.0 (`self.Negate` _returnvalue)) false false)
  (set `self.PercentageRoll` (`KismetMathLibrary.Abs` (/ (/ (* _returnvalue 100.0) (`self.MaxAileronPtich`)) 100.0))))

(fn `ResetElevator`
  (bind _maxelevatorpitch (`self.MaxElevatorPitch`))
  (bind _maxflapptich (`self.MaxFlapPtich`))
  (bind _returnvalue (`KismetMathLibrary.MapRangeClamped` (`self.CurrentPitch`) -1.0 1.0 _maxelevatorpitch (`self.Negate` _maxelevatorpitch)))
  (bind _returnvalue_2 (`KismetMathLibrary.MapRangeClamped` (`self.CurrentPitch`) -1.0 1.0 _maxflapptich (`self.Negate` _maxflapptich)))
  (bind _out (`self.Negate` _returnvalue))
  (set `self.TargetPitch` 0.0)
  (set `self.CurrentPitch` (`KismetMathLibrary.FInterpTo` (`self.CurrentPitch`) (`self.TargetPitch`) (`GameplayStatics.GetWorldDeltaSeconds`) 10.0))
  (`SceneComponent.K2_SetRelativeRotation` (`self.FlapL`) (`KismetMathLibrary.MakeRotator` 0.0 _returnvalue_2) false false)
  (`SceneComponent.K2_SetRelativeRotation` (`self.FlapR`) (`KismetMathLibrary.MakeRotator` 0.0 _returnvalue_2) false false)
  (`SceneComponent.K2_SetRelativeRotation` (`self.ElevatorL`) (`KismetMathLibrary.MakeRotator` 0.0 _out) false false)
  (`SceneComponent.K2_SetRelativeRotation` (`self.ElevatorR`) (`KismetMathLibrary.MakeRotator` 0.0 _out) false false)
  (set `self.PercentagePitch` (`KismetMathLibrary.Abs` (/ (/ (* _returnvalue 100.0) (`self.MaxElevatorPitch`)) 100.0))))

(fn `ResetRudder`
  (bind _returnvalue (`KismetMathLibrary.MapRangeClamped` (`self.CurrentYaw`) -1.0 1.0 (`self.maxRudderYaw`) (`self.Negate` (`self.maxRudderYaw`))))
  (set `self.TargetYaw` 0.0)
  (set `self.CurrentYaw` (`KismetMathLibrary.FInterpTo` (`self.CurrentYaw`) (`self.TargetYaw`) (`GameplayStatics.GetWorldDeltaSeconds`) 10.0))
  (`SceneComponent.K2_SetRelativeRotation` (`self.RudderL`) (`KismetMathLibrary.MakeRotator` 0.0 0.0 _returnvalue) false false)
  (`SceneComponent.K2_SetRelativeRotation` (`self.RudderR`) (`KismetMathLibrary.MakeRotator` 0.0 0.0 _returnvalue) false false)
  (set `self.percentageYaw` (`KismetMathLibrary.Abs` (/ (/ (* _returnvalue 100.0) (`self.maxRudderYaw`)) 100.0))))

(fn `RollAnimation`
  (params (DeltaSecond :type "Float (double-precision)") (Roll :type "Float (double-precision)"))
  (bind _maxaileronptich (`self.MaxAileronPtich`))
  (bind _maxaileronptich_2 (`self.MaxAileronPtich`))
  (bind _returnvalue (`KismetMathLibrary.MapRangeClamped` (`self.CurrentRoll`) -1.0 1.0 _maxaileronptich_2 (`self.Negate` _maxaileronptich_2)))
  (set `self.TargetRoll` Roll)
  (set `self.CurrentRoll` (`KismetMathLibrary.FInterpTo` (`self.CurrentRoll`) (`self.TargetRoll`) (`GameplayStatics.GetWorldDeltaSeconds`) 10.0))
  (`SceneComponent.K2_SetRelativeRotation` (`self.aileronL`) (`KismetMathLibrary.MakeRotator` 0.0 (`KismetMathLibrary.MapRangeClamped` (`self.CurrentRoll`) -1.0 1.0 _maxaileronptich (`self.Negate` _maxaileronptich))) false false)
  (`SceneComponent.K2_SetRelativeRotation` (`self.AileronR`) (`KismetMathLibrary.MakeRotator` 0.0 (`self.Negate` _returnvalue)) false false)
  (set `self.PercentageRoll` (`KismetMathLibrary.Abs` (/ (/ (* _returnvalue 100.0) (`self.MaxAileronPtich`)) 100.0))))

(fn `ThrottleInput`
  (bind _accelamount (`self.AccelAmount`))
  (if (`self.AccelUP`)
    (bind _result (`/Engine/EditorBlueprintResources/StandardMacros.IncrementInt` _accelamount)
      (:`  `
        (set `self.AccelAmount` (`KismetMathLibrary.Clamp` _result 0 100))))
    (elif (`self.AccelDown`)
      (bind _result_2 (`/Engine/EditorBlueprintResources/StandardMacros.DecrementInt` _accelamount)
        (:`  `
          (set `self.AccelAmount` (`KismetMathLibrary.Clamp` _result_2 0 100)))))))

(fn `UpdateThruster`
  (`NiagaraComponent.SetVariableVec3` (`self.LeftThrusterEffect`) "Attractor Position Offset" (`KismetMathLibrary.MakeVector` (`KismetMathLibrary.MapRangeClamped` (`KismetMathLibrary.Conv_IntToDouble` (`self.AccelAmount`)) 0.0 100.0 0.0 -500.0)))
  (`NiagaraComponent.SetVariableVec3` (`self.RightThrusterEffect`) "Attractor Position Offset" (`KismetMathLibrary.MakeVector` (`KismetMathLibrary.MapRangeClamped` (`KismetMathLibrary.Conv_IntToDouble` (`self.AccelAmount`)) 0.0 100.0 0.0 -500.0))))

(fn `UserConstructionScript`)

(fn `YawAnimation`
  (params (DeltaSecond :type "Float (double-precision)") (Yaw :type "Float (double-precision)"))
  (bind _returnvalue (`KismetMathLibrary.MapRangeClamped` (`self.CurrentYaw`) -1.0 1.0 (`self.maxRudderYaw`) (`self.Negate` (`self.maxRudderYaw`))))
  (set `self.TargetYaw` Yaw)
  (set `self.CurrentYaw` (`KismetMathLibrary.FInterpTo` (`self.CurrentYaw`) (`self.TargetYaw`) (`GameplayStatics.GetWorldDeltaSeconds`) 10.0))
  (`SceneComponent.K2_SetRelativeRotation` (`self.RudderL`) (`KismetMathLibrary.MakeRotator` 0.0 0.0 _returnvalue) false false)
  (`SceneComponent.K2_SetRelativeRotation` (`self.RudderR`) (`KismetMathLibrary.MakeRotator` 0.0 0.0 _returnvalue) false false)
  (set `self.percentageYaw` (`KismetMathLibrary.Abs` (/ (/ (* _returnvalue 100.0) (`self.maxRudderYaw`)) 100.0))))