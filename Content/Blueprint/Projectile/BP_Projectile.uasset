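; BP_Projectile is a short-lived explosive projectile that acts when its Sphere component hits something.
; On impact it spawns and triggers an FS_MasterField at the hit point, likely to fracture destructibles.
; It gives the hit component a fixed-direction velocity-change impulse and makes it ignore Pawn collision.
; It then spawns a normal-aligned explosion effect and sound, and destroys itself.
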(event `self.ReceiveBeginPlay`
  (`self.SetLifeSpan` 3.0))

(event `self.Sphere.OnComponentHit`
  (params (HitComponent :type "PrimitiveComponent Object Reference") (OtherActor :type "Actor Object Reference") (OtherComp :type "PrimitiveComponent Object Reference") (NormalImpulse :type "Vector Structure") (Hit :type "HitResult Structure (by ref)"))
  (set `self.Hit Impact Normal` Hit_ImpactNormal)
  (set `self.Hit Location` Hit_Location)
  (bind _returnvalue (`|SpawnActorFromClass` "/Engine/EditorResources/FieldNodes/FS_MasterField.FS_MasterField_C" (`KismetMathLibrary.MakeTransform` Hit_Location) "Undefined" "MultiplyWithRoot" null null))
  (set `/Engine/EditorResources/FieldNodes/FS_MasterField.ActivationType` "NewEnumerator4" _returnvalue)
  (`/Engine/EditorResources/FieldNodes/FS_MasterField.CE_Trigger` _returnvalue)
  (`PrimitiveComponent.AddImpulse` OtherComp (5000.0 5000.0 0.0) "None" true)
  (`PrimitiveComponent.SetCollisionResponseToChannel` OtherComp "ECC_Pawn" "ECR_Ignore")
  (`NiagaraFunctionLibrary.SpawnSystemAtLocation` "/Game/Blueprint/Projectile/Niagara/NS_Explosion.NS_Explosion" (`self.Hit Location`) (`KismetMathLibrary.MakeRotFromZ` (`self.Hit Impact Normal`)))
  (`GameplayStatics.SpawnSoundAtLocation` "/Game/StarterContent/Audio/Explosion_Cue.Explosion_Cue" (`self.Hit Location`) (struct) 1.0 1.0 0.0 "/Game/Blueprint/Tank/SoundTank/ATT_explosion.ATT_explosion" null)
  (`self.K2_DestroyActor`))

(fn `UserConstructionScript`)